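; BP_Surcharge_zone is an interactable actor that refills part of the player's surcharge gauge once, then disappears.
; Its Sphere overlap events enable input when a BP_Character enters and disable it on exit, so the Action input works only nearby.
; Pressing Action disables input, adds a fixed amount to JaugeSurchargePercent on BP_GameInstance, clamped as a percentage, and destroys the actor after a short delay.
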(event OnComponentBeginOverlap(Sphere)
  (params (OverlappedComponent :type Primitive%20Component%20Object%20Reference) (OtherActor :type Actor%20Object%20Reference) (OtherComp :type Primitive%20Component%20Object%20Reference) (OtherBodyIndex :type Integer) (bFromSweep :type Boolean) (SweepResult :type Hit%20Result%20Structure%20%28by%20ref%29))
  ;[1 1 1] player near, enable input
  (if (.bSuccess (Utilities|Casting|CastToBP_Character OtherActor))
    (Input|EnableInput (Game|GetPlayerController 0))))

(event OnComponentEndOverlap(Sphere)
  (params (OverlappedComponent :type Primitive%20Component%20Object%20Reference) (OtherActor :type Actor%20Object%20Reference) (OtherComp :type Primitive%20Component%20Object%20Reference) (OtherBodyIndex :type Integer))
  ;[1 1 1] player far, cannot take surcharge zone
  (if (.bSuccess (Utilities|Casting|CastToBP_Character OtherActor))
    (Input|DisableInput (Game|GetPlayerController 0))))

(event Input|ActionEvents|InputActionAction
  (params (Key :type Key%20Structure))
  (bind _returnvalue (Game|GetGameInstance))
  (bind _asbp_game_instance (Utilities|Casting|CastToBP_GameInstance _returnvalue))
  ;[1 1 1] player took surcharge zone
  (:Pressed
    (Input|DisableInput (Game|GetPlayerController 0))
    (Variables|/Game/Blueprints/BP_GameInstance.BP_GameInstance_C|SetJaugeSurchargePercent _asbp_game_instance (Math|Float|Clamp(Float) (+ (Variables|/Game/Blueprints/BP_GameInstance.BP_GameInstance_C|GetJaugeSurchargePercent _asbp_game_instance) 5e+01) 0.0 1e+02))
    (Utilities|FlowControl|Delay 0.5)
    (Actor|DestroyActor)))

(fn ConstructionScript)