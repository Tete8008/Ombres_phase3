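; BP_spot is a light actor that animates its rotation when play begins, sweeping in yaw and tilting in pitch.
; A timeline with play rate 1/Time feeds two tracks into separate rotator lerps from the stored Rotation, one toward a 360-degree yaw offset, the other toward an Inclinaison pitch offset.
; Each update applies both with roll at zero, and the finished event saves the actor's final rotation.
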(event EventBeginPlay
  ;[1 1 1] Durée de la timeline
  (Components|Timeline|SetPlayRate (Variables|Default|GetTimeline_0) (/ 1.0 (Variables|Default|GetTime)))
  (bind (_direction _newtrack_0 _newtrack_1) (Timeline|Timeline_0 Play)
    (:Update
      ;[1 1 1] Set la rotation de l'actor en fonction des lerps
      (Transformation|SetActorRotation (Math|Rotator|MakeRotator 0.0 (.Pitch (Math|Rotator|BreakRotator (Math|Rotator|Lerp(Rotator) (Variables|Default|GetRotation) (Math|Rotator|MakeRotator (.Roll (Math|Rotator|BreakRotator (Variables|Default|GetRotation))) (+ (.Pitch (Math|Rotator|BreakRotator (Variables|Default|GetRotation))) (Variables|Default|GetInclinaison)) (.Yaw (Math|Rotator|BreakRotator (Variables|Default|GetRotation)))) _newtrack_1))) (.Yaw (Math|Rotator|BreakRotator (Math|Rotator|Lerp(Rotator) (Variables|Default|GetRotation) (Math|Rotator|MakeRotator (.Roll (Math|Rotator|BreakRotator (Variables|Default|GetRotation))) (.Pitch (Math|Rotator|BreakRotator (Variables|Default|GetRotation))) (+ (.Yaw (Math|Rotator|BreakRotator (Variables|Default|GetRotation))) 3.6e+02)) _newtrack_0))))))
    (:Finished
      ;[1 1 1] Set la rotation actuelle de la light
      (Variables|Default|SetRotation (Transformation|GetActorRotation)))))

(fn ConstructionScript)