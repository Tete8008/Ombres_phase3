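; BP_Functions holds a projectile math helper, CalculateVelocity, which returns the launch velocity needed to travel from a start position to a destination in a given duration.
; X and Y use constant speed, displacement divided by duration, while Z adds compensation for gravitational drop.
; Gravity is hardcoded at 981 units per second squared rather than read from the world, and drag is not modeled.
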(fn CalculateVelocity
  (params (Duration :type Float%20%28single-precision%29) (StartPosition :type Vector) (DestinationPosition :type Vector))
  (bind (_x _y _z) (Math|Vector|BreakVector DestinationPosition))
  (bind (_x_2 _y_2 _z_2) (Math|Vector|BreakVector StartPosition))
  (LocalVariables|SetLocalDuration Duration)
  (return (Math|Vector|MakeVector (/ (- _x _x_2) (LocalVariables|GetLocalDuration)) (/ (- _y _y_2) (LocalVariables|GetLocalDuration)) (/ (- _z (+ _z_2 (* (Math|Float|Square (LocalVariables|GetLocalDuration)) -0.5 981.0))) (LocalVariables|GetLocalDuration)))))