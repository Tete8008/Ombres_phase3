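; BP_Grue02 is a crane actor that swings around when something overlaps its Box trigger.
; BeginPlay caches the actor's rotation as the starting point.
; The overlap plays the Rotation timeline forward at half speed, lerping the Grue component's world rotation to 60° more yaw, with no reverse.
; The graph comment says 90°, but the code adds 60°.
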(event OnComponentBeginOverlap(Box)
  (params (OverlappedComponent :type Primitive%20Component%20Object%20Reference) (OtherActor :type Actor%20Object%20Reference) (OtherComp :type Primitive%20Component%20Object%20Reference) (OtherBodyIndex :type Integer) (bFromSweep :type Boolean) (SweepResult :type Hit%20Result%20Structure%20%28by%20ref%29))
  (bind _inirot (Variables|Default|GetIniRot))
  (bind (_roll _pitch _yaw) (Math|Rotator|BreakRotator _inirot))
  ;[1 1 1] Fait tourner la grue de 90°
  (Components|Timeline|SetPlayRate (Variables|Default|GetRotation) (/ 1.0 2.0))
  (bind _newtrack_0 (Timeline|Rotation Play)
    (:Update
      (Transformation|SetWorldRotation (Variables|Default|GetGrue) (Math|Rotator|Lerp(Rotator) _inirot (Math|Rotator|MakeRotator _roll _pitch (+ _yaw 6e+01)) _newtrack_0) false false))))

(event EventBeginPlay
  ;[1 1 1] Fait tourner la grue de 90°
  (Variables|Default|SetIniRot (Transformation|GetActorRotation)))

(fn ConstructionScript)