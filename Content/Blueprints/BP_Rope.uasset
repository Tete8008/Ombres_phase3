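; BP_Rope is a physics cable that the player character can grab and hang from by the left hand.
; BeginPlay adds an overlap box per cable particle, and Tick moves each box to follow the simulation.
; A capsule overlap attaches the character, picks a particle by height and briefly applies twice the player's velocity as cable force.
; Tick pins the player's hand to that particle, while DisableCollisions blocks re-grabbing for one second.
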(event Custom|BoxOverlap
  (params (OverlappedComponent :type Primitive%20Component%20Object%20Reference) (OtherActor :type Actor%20Object%20Reference) (OtherComp :type Primitive%20Component%20Object%20Reference) (OtherBodyIndex :type Integer) (bFromSweep :type Boolean) (SweepResult :type Hit%20Result%20Structure%20%28by%20ref%29))
  (bind _cable (Variables|Default|GetCable))
  (bind _locations (Class|CableComponent|GetCableParticleLocations _cable))
  ;[1 1 1] On overlap
  (if (Variables|Default|GetCollisionsEnabled)
    (Utilities|Casting|CastToCapsuleComponent OtherComp)
    (bind _asbp_character (Utilities|Casting|CastToBP_Character OtherActor))
    (if (not (Variables|/Game/Blueprints/BP_Character.BP_Character_C|GetAttachedToRope _asbp_character))
      (Variables|/Game/Blueprints/BP_Character.BP_Character_C|SetAttachedToRope _asbp_character true)
      (Variables|/Game/Blueprints/BP_Character.BP_Character_C|SetRope _asbp_character self)
      (Game|Feedback|ClientStopCameraShake (Game|GetPlayerController 0) "/Script/Engine.CameraShake" true)
      (bind _output_get (Variables|Default|SetParticleAttachedIndex (Math|Float|Round (* (/ (- (.Z (Math|Vector|BreakVector (Utilities|Array|Get(acopy) _locations))) (.Z (Math|Vector|BreakVector (Transformation|GetWorldLocation OverlappedComponent)))) (Variables|/Script/CableComponent.CableComponent|GetCableLength (Variables|Default|GetCable))) (Math|Conversions|ToFloat(Integer) (- (Utilities|Array|Length _locations) 1))))))
      (Variables|/Script/CableComponent.CableComponent|SetCableForce (Variables|Default|GetCable) (* (Transformation|GetVelocity (Game|GetPlayerCharacter 0)) 2.0))
      (Utilities|Time|SetTimerbyEvent (delegate Custom|RemoveForce) (/ (Math|Conversions|ToFloat(Integer) _output_get) 2e+01)))))

(event Custom|BoxOverlapEnd
  (params (OverlappedComponent :type Primitive%20Component%20Object%20Reference) (OtherActor :type Actor%20Object%20Reference) (OtherComp :type Primitive%20Component%20Object%20Reference) (OtherBodyIndex :type Integer))
  ;[1 1 1] At start we add collision boxes along the rope
)

(event Custom|DisableCollisions
  ;[1 1 1] Disable collisions for 1 second to prevent being stuck on the rope
  (Variables|Default|SetCollisionsEnabled false)
  (Utilities|Time|SetTimerbyEvent (delegate Custom|ReEnableCollisions) 1.0))

(event Custom|ReEnableCollisions
  ;[1 1 1] Disable collisions for 1 second to prevent being stuck on the rope
  (Variables|Default|SetCollisionsEnabled true))

(event Custom|RemoveForce
  ;[1 1 1] On overlap
  (Variables|/Script/CableComponent.CableComponent|SetCableForce (Variables|Default|GetCable) "0, 0, 0"))

(event EventTick
  (params (DeltaSeconds :type Float%20%28single-precision%29))
  (bind _returnvalue (Game|GetPlayerCharacter 0))
  (bind _cable (Variables|Default|GetCable))
  (bind _locations (Class|CableComponent|GetCableParticleLocations _cable))
  (bind _asbp_character (Utilities|Casting|CastToBP_Character _returnvalue))
  ;[1 1 1] Every frame we update the box collisions along the rope, abd if the player is attached, we update his position too
  (for _index (range 0 (- (Utilities|Array|Length _locations) 1))
    (Transformation|SetWorldLocation (Utilities|Array|Get(acopy) (Variables|Default|GetBoxCollisions) _index) (Utilities|Array|Get(acopy) _locations _index) false false))
  (if (!= (Variables|Default|GetParticleAttachedIndex) -1)
    (Transformation|SetActorLocation _asbp_character (- (Utilities|Array|Get(acopy) (Class|CableComponent|GetCableParticleLocations (Variables|Default|GetCable)) (Variables|Default|GetParticleAttachedIndex)) (- (Transformation|GetSocketLocation (Variables|/Script/Engine.Character|GetMesh _asbp_character) "LeftHand") (Transformation|GetActorLocation _asbp_character))) false false)))

(event EventBeginPlay
  (bind _cable (Variables|Default|GetCable))
  (bind _locations (Class|CableComponent|GetCableParticleLocations _cable))
  ;[1 1 1] At start we add collision boxes along the rope
  (Physics|SetSimulatePhysics _cable true)
  (for _array_element _locations
    (bind _returnvalue (AddComponent|AddBoxComponent true (Math|Transform|MakeTransform _array_element)))
    (Collision|SetCollisionResponsetoAllChannels _returnvalue "ECR_Overlap")
    (Collision|BindEventtoOnComponentBeginOverlap _returnvalue (delegate Custom|BoxOverlap))
    (Collision|BindEventtoOnComponentEndOverlap _returnvalue (delegate Custom|BoxOverlapEnd))
    (Transformation|SetRelativeScale3D _returnvalue (* "1.000000,1.000000,1.000000" (/ 1.0 (Math|Conversions|ToFloat(Integer) (Utilities|Array|Length _locations)))))
    (Utilities|Array|Add (Variables|Default|GetBoxCollisions) _returnvalue)))

(fn ConstructionScript)