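; BP_SplineLampadaire is a spline-driven placement actor that lines up streetlamps (BP_Lampadaire) along a path.
; The construction script adds a child actor component at each spline point, using the point's local location and rotation.
; Each spawned lamp is cast to BP_Lampadaire and stored in the Lampadaire array.
; The event graph holds no runtime logic.
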(event EventBeginPlay)

(event Collision|EventActorBeginOverlap
  (params (OtherActor :type Actor%20Object%20Reference)))

(event EventTick
  (params (DeltaSeconds :type Float%20%28single-precision%29)))

(fn ConstructionScript
  (bind _spline (Variables|Default|GetSpline))
  (bind _output_get (Variables|Default|SetNBSplinePoint (- (Spline|GetNumberOfSplinePoints (Variables|Default|GetSpline)) 1)))
  (for _index (range 0 _output_get)
    (Variables|Default|SetIndexOfLoop _index)
    (bind _returnvalue (AddComponent|AddChildActorComponent false (Math|Conversions|ToTransform(Vector) (Spline|GetLocationatSplinePoint _spline (Variables|Default|GetIndexOfLoop) "Local"))))
    (ChildActorComponent|SetChildActorClass _returnvalue "/Game/Blueprints/BP_Lampadaire.BP_Lampadaire_C")
    (bind _asbp_lampadaire (Utilities|Casting|CastToBP_Lampadaire (Variables|/Script/Engine.ChildActorComponent|GetChildActor _returnvalue)))
    (Utilities|Array|Add (Variables|Default|GetLampadaire) _asbp_lampadaire)
    (Transformation|SetRelativeRotation _returnvalue (Spline|GetRotationatSplinePoint _spline (Variables|Default|GetIndexOfLoop) "Local") false false)))