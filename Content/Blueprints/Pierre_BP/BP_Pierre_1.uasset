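; BP_Pierre_1 is a skeletal mesh Blueprint that loops an idle animation and reacts to a PowerOn event.
; The construction script creates a dynamic material instance with Pouvoir_01 raised and the other two Pouvoir parameters zeroed.
; PowerOn plays the attack animation, waits briefly, then sets a negative play rate and restarts it.
; The idle call follows immediately, overriding that replay, and the play rate is never restored.
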(event Custom|PowerOn
  (bind _skeletalmesh (Variables|Default|GetSkeletalMesh))
  (Components|Animation|PlayAnimation _skeletalmesh "/Game/SM_main/anim_2/attack_Anim.attack_Anim" false)
  (Utilities|FlowControl|Delay 1.0)
  (Components|Timeline|SetPlayRate _skeletalmesh -1.0)
  (Components|Animation|PlayAnimation _skeletalmesh "/Game/SM_main/anim_2/attack_Anim.attack_Anim" false)
  (Components|Animation|PlayAnimation _skeletalmesh "/Game/SM_main/anim_2/idel_Anim.idel_Anim" true))

(event EventBeginPlay
  (Components|Animation|PlayAnimation (Variables|Default|GetSkeletalMesh) "/Game/SM_main/anim_2/idel_Anim.idel_Anim" true))

(fn ConstructionScript
  (bind _returnvalue (Rendering|Material|CreateDynamicMaterialInstance (Variables|Default|GetSkeletalMesh) 0 0 "None" :!class /Script/Engine.PrimitiveComponent))
  (Rendering|Material|SetMaterial (Variables|Default|GetSkeletalMesh) 0 _returnvalue)
  (Rendering|Material|SetScalarParameterValue _returnvalue "Pouvoir_01" 1e+02 :!class /Script/Engine.MaterialInstanceDynamic)
  (Rendering|Material|SetScalarParameterValue _returnvalue "Pouvoir_02" 0.0 :!class /Script/Engine.MaterialInstanceDynamic)
  (Rendering|Material|SetScalarParameterValue _returnvalue "Pouvoir_03" 0.0 :!class /Script/Engine.MaterialInstanceDynamic))