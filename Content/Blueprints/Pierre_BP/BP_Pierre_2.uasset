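; Pierre_2 actor Blueprint with a skeletal mesh that plays its main attack animation when powered on.
; The PowerOn event plays Main_attack_Anim once on the mesh, without looping.
; The construction script creates a dynamic material instance on the first material slot and initializes three "Pouvoir" power parameters, with only the third set non-zero.
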(event Custom|PowerOn
  (Components|Animation|PlayAnimation (Variables|Default|GetSkeletalMesh) "/Game/Blueprints/Mainanim/main_attack_Anim.main_attack_Anim" false))

(event EventBeginPlay)

(event Collision|EventActorBeginOverlap
  (params (OtherActor :type Actor%20Object%20Reference)))

(event EventTick
  (params (DeltaSeconds :type Float%20%28single-precision%29)))

(fn ConstructionScript
  (bind _returnvalue (Rendering|Material|CreateDynamicMaterialInstance (Variables|Default|GetSkeletalMesh) 0 0 "None" :!class /Script/Engine.PrimitiveComponent))
  (Rendering|Material|SetMaterial (Variables|Default|GetSkeletalMesh) 0 _returnvalue)
  (Rendering|Material|SetScalarParameterValue _returnvalue "Pouvoir_01" 0.0 :!class /Script/Engine.MaterialInstanceDynamic)
  (Rendering|Material|SetScalarParameterValue _returnvalue "Pouvoir_02" 0.0 :!class /Script/Engine.MaterialInstanceDynamic)
  (Rendering|Material|SetScalarParameterValue _returnvalue "Pouvoir_03" 1e+02 :!class /Script/Engine.MaterialInstanceDynamic))