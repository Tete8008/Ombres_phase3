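; Bomber plane actor with two scripted flight events: a bombing pass (ThrowingFire) and a crash (Mayday).
; Timelines move and rotate the Scene component along splines at constant velocity with a -90 yaw offset, with play rates derived from duration variables.
; Mayday chains the Start path into the Crash path, then plays a 2D explosion sound.
; A propeller-spin timeline update exists, but nothing starts it.
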(event Custom|Mayday
  (bind _crash (Variables|Spline|GetCrash))
  (bind _start (Variables|Spline|GetStart))
  ;[0.03086 0.5887 1] L'avion s'écrase
  (Components|Timeline|SetPlayRate (Variables|Default|GetDepart) (/ 1.0 (Variables|Duration|GetTimeStart)))
  (bind _newtrack_0 (Timeline|Depart Play)
    (:Update
      (Transformation|SetWorldLocationAndRotation (Variables|Avion|GetScene) (Spline|GetLocationatTime _start _newtrack_0 "World" true) (Math|Rotator|MakeRotator (.Roll (Math|Rotator|BreakRotator (Class|SplineComponent|GetRotationatTime _start _newtrack_0 "World" true))) (.Pitch (Math|Rotator|BreakRotator (Class|SplineComponent|GetRotationatTime _start _newtrack_0 "World" true))) (+ (.Yaw (Math|Rotator|BreakRotator (Class|SplineComponent|GetRotationatTime _start _newtrack_0 "World" true))) -9e+01)) false false))
    (:Finished
      (Components|Timeline|SetPlayRate (Variables|Default|GetCrashplane) (/ 1.0 (Variables|Duration|GetTimeCrash)))
      (bind _newtrack_0_2 (Timeline|Crashplane Play)
        (:Update
          (Transformation|SetWorldLocationAndRotation (Variables|Avion|GetScene) (Spline|GetLocationatTime _crash _newtrack_0_2 "World" true) (Math|Rotator|MakeRotator (.Roll (Math|Rotator|BreakRotator (Class|SplineComponent|GetRotationatTime _crash _newtrack_0_2 "World" true))) (.Pitch (Math|Rotator|BreakRotator (Class|SplineComponent|GetRotationatTime _crash _newtrack_0_2 "World" true))) (+ (.Yaw (Math|Rotator|BreakRotator (Class|SplineComponent|GetRotationatTime _crash _newtrack_0_2 "World" true))) -9e+01)) false false))
        (:Finished
          (Audio|PlaySound2D "/Game/StarterContent/Audio/Explosion_Cue.Explosion_Cue" 1.0 1.0 0.0 0 0))))))

(event Custom|Throwing%20Fire
  (bind _bombardement (Variables|Spline|GetBombardement))
  ;[1 0.2737 0.3736] Lance la bombe
  (Components|Timeline|SetPlayRate (Variables|Default|GetBombe) (/ 1.0 (Variables|Duration|GetTimeBombardement)))
  (bind _newtrack_0 (Timeline|Bombe Play)
    (:Update
      (Transformation|SetWorldLocationAndRotation (Variables|Avion|GetScene) (Spline|GetLocationatTime _bombardement _newtrack_0 "World" true) (Math|Rotator|MakeRotator (.Roll (Math|Rotator|BreakRotator (Class|SplineComponent|GetRotationatTime _bombardement _newtrack_0 "World" true))) (.Pitch (Math|Rotator|BreakRotator (Class|SplineComponent|GetRotationatTime _bombardement _newtrack_0 "World" true))) (+ (.Yaw (Math|Rotator|BreakRotator (Class|SplineComponent|GetRotationatTime _bombardement _newtrack_0 "World" true))) -9e+01)) false false))))

(fn ConstructionScript)