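; Enemy AI character that wanders the navmesh, chases the player on sight and can leap to catch them.
; AIMoveTo loops drive roaming and pursuit, with pawn sensing resetting a lost-sight timer that leads to a confused pause before roaming resumes.
; Tick tracks catching range, halting a chasing enemy and registering it with BP_Character.
; Launches handle navlink jumps and the catch leap; hitting the player only prints a message.
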(event OnSeePawn(PawnSensing)
  (params (Pawn :type Pawn%20Object%20Reference))
  ;[1 1 1] Chase character
  (if (Math|Boolean|ANDBoolean (Variables|Default|GetCanMove) (not (AI|Components|NavMovement|IsFalling (Variables|Character|GetCharacterMovement))) (not (Variables|Default|GetInRangeOfPlayer)))
    (Variables|Default|SetTimeSinceCharacterWasSeen 0.0)
    (Variables|/Script/Engine.CharacterMovementComponent|SetMaxWalkSpeed (Variables|Character|GetCharacterMovement) (Variables|Default|GetRunSpeed))
    (Utilities|Casting|CastToBP_Character Pawn)
    (if (not (Variables|Default|GetMovingTowardsCharacter))
      (AI|AIMoveTo self "0, 0, 0" (Game|GetPlayerCharacter 0) 5.0 false :!label _label
        (:then
          (Variables|Default|SetMovingTowardsCharacter true))
        (:OnSuccess
          (Utilities|FlowControl|Delay 0.1 :!label _label_2)
          (if (and (not (Variables|Default|GetJumping)) (not (Variables|Default|GetInRangeOfPlayer)))
            (goto _label)
            (else
              (goto _label_2))))
        (:OnFail
          (goto _label_2))))))

(event Custom|AIJump
  (params (Velocity :type Vector))
  ;[1 1 1] NavLink jump
  (Character|LaunchCharacter Velocity true true)
  (Variables|Default|SetJumping true))

(event Custom|ResearchState
  ;[1 1 1] Research state
  (if (Variables|Default|GetCanMove)
    (Variables|/Script/Engine.CharacterMovementComponent|SetMaxWalkSpeed (Variables|Character|GetCharacterMovement) (Variables|Default|GetWalkSpeed))
    (if (not (Variables|Default|GetMovingTowardsCharacter)) :!label _label
      (AI|AIMoveTo self (.RandomLocation (Class|NavigationSystemV1|GetRandomPointinNavigableRadius (Transformation|GetActorLocation) 1e+04 0 0)) 0 5.0 false
        (:OnSuccess
          _)
        (:OnFail
          _))
      (Utilities|FlowControl|Delay 3.0)
      (goto _label))))

(event Custom|ConfusedState
  (bind _self self)
  ;[1 1 1] Confus
  (Variables|Default|SetMovingTowardsCharacter false)
  (AI|AIMoveTo _self "0, 0, 0" _self 5.0 false
    (:OnSuccess
      _)
    (:OnFail
      _))
  (Utilities|Time|SetTimerbyEvent (delegate Custom|ResearchState) (Variables|Default|GetConfusedDuration)))

(event Custom|CatchPlayer
  (bind _velocity (CallFunction|CalculateVelocity 0.5 (Transformation|GetActorLocation) (Transformation|GetActorLocation (Game|GetPlayerCharacter 0))))
  (Character|LaunchCharacter _velocity true true))

(event Custom|FindPlaceAroundPlayer)

(event Custom|PrepareJumpingOnPlayer
  (bind _self self)
  (if (Variables|Default|GetMovingTowardsCharacter)
    (AI|AIMoveTo _self "0, 0, 0" _self 5.0 false
      (:OnSuccess
        _)
      (:OnFail
        _))
    (Default|AddEnemyinRange (Variables|Default|GetPlayer) self)))

(event Custom|GetOutOfRange
  (if (Variables|Default|GetMovingTowardsCharacter)
    (Default|RemoveEnemyinRange (Variables|Default|GetPlayer) self)))

(event EventBeginPlay
  ;[1 1 1] START
  (Variables|Default|SetInitialMaterial (Rendering|Material|GetMaterial (Variables|Character|GetMesh) 2))
  (Variables|Default|SetPlayer (.AsBP%20Character (Utilities|Casting|CastToBP_Character (Game|GetPlayerCharacter 0))))
  (CallFunction|ResearchState))

(event Collision|EventHit
  (params (MyComp :type Primitive%20Component%20Object%20Reference) (Other :type Actor%20Object%20Reference) (OtherComp :type Primitive%20Component%20Object%20Reference) (bSelfMoved :type Boolean) (HitLocation :type Vector :default "0, 0, 0") (HitNormal :type Vector :default "0, 0, 0") (NormalImpulse :type Vector :default "0, 0, 0") (Hit :type Hit%20Result%20Structure%20%28by%20ref%29))
  (Utilities|Casting|CastToBP_Character Other
    (:then
      (Development|PrintString "You got caught noob"))
    (:CastFailed
      (if (Variables|Default|GetJumping)
        (Variables|Default|SetJumping false)))))

(event EventTick
  (params (DeltaSeconds :type Float%20%28single-precision%29))
  ;[1 1 1] EVENT TICK
  (bind _distance (CallFunction|CalculateDistancetoPlayer))
  (if (Math|Boolean|NotEqual(Boolean) (<= _distance (Variables|Default|GetCatchingRange)) (Variables|Default|GetInRangeOfPlayer))
    (Variables|Default|SetInRangeOfPlayer (<= _distance (Variables|Default|GetCatchingRange)))
    (if (<= _distance (Variables|Default|GetCatchingRange))
      (CallFunction|PrepareJumpingonPlayer)
      (else
        (CallFunction|GetOutOfRange)))
    (else
      (Variables|Default|SetInRangeOfPlayer (<= _distance (Variables|Default|GetCatchingRange)))
      (if (and (Variables|Default|GetMovingTowardsCharacter) (not (Variables|Default|GetInRangeOfPlayer)))
        (bind _output_get (Variables|Default|SetTimeSinceCharacterWasSeen (+ DeltaSeconds (Variables|Default|GetTimeSinceCharacterWasSeen))))
        (if (>= _output_get (Variables|Default|GetLostSightButStillChasingDuration))
          (CallFunction|ConfusedState))))))

(fn ConstructionScript)

(fn CalculateDistancetoPlayer
  (return (Math|Float|Sqrt (Math|Vector|VectorLengthSquared (- (Transformation|GetActorLocation) (Transformation|GetActorLocation (Variables|Default|GetPlayer)))))))