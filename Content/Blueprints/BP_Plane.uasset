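; BP_Plane is a plane actor that flies along a spline path from BeginPlay.
; The Vol timeline, with its play rate set from Duration, samples the spline at constant velocity to set the world location and rotation of Scene1, offsetting yaw by -90 degrees.
; A second timeline meant to spin the propeller is left unconnected and never runs.
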(event EventBeginPlay
  (bind _spline (Variables|Default|GetSpline))
  ;[1 1 1] Vol
  (Components|Timeline|SetPlayRate (Variables|Default|GetVol) (/ 1.0 (Variables|Default|GetDuration)))
  (bind _newtrack_0 (Timeline|Vol Play)
    (:Update
      (Transformation|SetWorldLocationAndRotation (Variables|Default|GetScene1) (Spline|GetLocationatTime _spline _newtrack_0 "World" true) (Math|Rotator|MakeRotator (.Roll (Math|Rotator|BreakRotator (Class|SplineComponent|GetRotationatTime _spline _newtrack_0 "World" true))) (.Pitch (Math|Rotator|BreakRotator (Class|SplineComponent|GetRotationatTime _spline _newtrack_0 "World" true))) (+ (.Yaw (Math|Rotator|BreakRotator (Class|SplineComponent|GetRotationatTime _spline _newtrack_0 "World" true))) -9e+01)) false false))))

(fn ConstructionScript)