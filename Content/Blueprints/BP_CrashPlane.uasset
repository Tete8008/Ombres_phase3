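; Plane actor that plays a crash by flying along a spline when its Crash event fires.
; A timeline, with play rate set to stretch its duration, samples the spline at constant velocity to set the plane component's world location and rotation, with a yaw offset to align it.
; A second timeline meant to spin the propeller is present but never runs.
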(event Custom|Crash
  (bind _spline (Variables|Default|GetSpline))
  ;[1 1 1] Crash d'avion en suivant la spline
  (Components|Timeline|SetPlayRate (Variables|Default|GetTimeline_0) (/ 1.0 2.7))
  (bind _newtrack_0 (Timeline|Timeline_0 Play)
    (:Update
      (Transformation|SetWorldLocationAndRotation (Variables|Default|GetScene1) (Spline|GetLocationatTime _spline _newtrack_0 "World" true) (Math|Rotator|MakeRotator (.Roll (Math|Rotator|BreakRotator (Class|SplineComponent|GetRotationatTime _spline _newtrack_0 "World" true))) (.Pitch (Math|Rotator|BreakRotator (Class|SplineComponent|GetRotationatTime _spline _newtrack_0 "World" true))) (+ (.Yaw (Math|Rotator|BreakRotator (Class|SplineComponent|GetRotationatTime _spline _newtrack_0 "World" true))) -9e+01)) false false))))

(fn ConstructionScript)