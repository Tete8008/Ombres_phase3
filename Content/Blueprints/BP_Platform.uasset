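; BP_Platform is a platform actor that toggles the visibility of its PPower1Platforme component when a BP_Character overlaps it.
; While the Spawned flag is false, begin overlap hides the component and its children, and end overlap shows them again.
; Once Spawned is true, both overlap events leave visibility untouched; this graph only reads that flag and never sets it.
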(event Collision|EventActorBeginOverlap
  (params (OtherActor :type Actor%20Object%20Reference))
  (if (not (Variables|Default|GetSpawned))
    (if (.bSuccess (Utilities|Casting|CastToBP_Character OtherActor))
      (Rendering|SetVisibility (Variables|Default|GetP_Power1_platforme) false true))))

(event Collision|EventActorEndOverlap
  (params (OtherActor :type Actor%20Object%20Reference))
  (if (not (Variables|Default|GetSpawned))
    (if (.bSuccess (Utilities|Casting|CastToBP_Character OtherActor))
      (Rendering|SetVisibility (Variables|Default|GetP_Power1_platforme) true true))))

(fn ConstructionScript)