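; BP_Geyser is a one-shot launcher that pushes the player character when it overlaps the geyser's sphere.
; It adds a Force-scaled push to BP_Character's movement component along the actor's up vector, then destroys itself.
; When the up vector is near horizontal or points downward, part of the actor's right vector is blended into the push direction.
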(event OnComponentBeginOverlap(Sphere)
  (params (OverlappedComponent :type Primitive%20Component%20Object%20Reference) (OtherActor :type Actor%20Object%20Reference) (OtherComp :type Primitive%20Component%20Object%20Reference) (OtherBodyIndex :type Integer) (bFromSweep :type Boolean) (SweepResult :type Hit%20Result%20Structure%20%28by%20ref%29))
  (bind _returnvalue (Transformation|GetActorUpVector))
  (if (== OtherActor (Game|Player|GetPlayerPawn 0))
    (Utilities|FlowControl|DoOnce false
      (:Completed
        (bind _asbp_character (Utilities|Casting|CastToBP_Character OtherActor))
        (if (>= (.Z (Math|Vector|BreakVector _returnvalue)) 0.1)
          (Physics|AddForce (Variables|/Script/Engine.Character|GetCharacterMovement _asbp_character) (* _returnvalue (Variables|Default|GetForce)))
          (else
            (Physics|AddForce (Variables|/Script/Engine.Character|GetCharacterMovement _asbp_character) (* (+ _returnvalue (* (Transformation|GetActorRightVector) 0.6)) (Variables|Default|GetForce)))))
        (Actor|DestroyActor)))))

(event Collision|EventActorBeginOverlap
  (params (OtherActor :type Actor%20Object%20Reference)))

(event EventTick
  (params (DeltaSeconds :type Float%20%28single-precision%29)))

(fn ConstructionScript)