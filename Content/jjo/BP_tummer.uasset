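; BP_tummer is a test Blueprint for a ramp-placement ability on the A key, though its ramp spawn class is unset.
; While A is held, a timeline traces from the camera, spawning once then repositioning the ramp along the surface normal and camera direction.
; Releasing A stops positioning and destroys the ramp four seconds later.
; Unconnected graphs hold similar trace-and-spawn logic for BP_TimeBubble and a timed geyser.
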(event EventBeginPlay
  ;[1 1 1] Bulle temporel
)

(event Input|KeyboardEvents|A
  (params (Key :type Key%20Structure))
  (bind _camera (Variables|Default|GetCamera))
  (bind _camera_2 (Variables|Default|GetCamera))
  (bind _returnvalue (Transformation|GetWorldRotation _camera_2))
  (bind _returnvalue_2 (Transformation|GetWorldLocation _camera))
  (:Pressed
    ;[1 1 1] rampe
    (Timeline|Timeline_0 Play
      (:Update
        (Utilities|FlowControl|Sequence
          (:then_0
            (bind _outhit (Collision|LineTraceByChannel _returnvalue_2 (+ _returnvalue_2 (* (Math|Vector|GetForwardVector (Transformation|GetWorldRotation _camera)) 1e+05)) "TraceTypeQuery2" false 0 "ForDuration" true "(R=1.000000,G=0.000000,B=0.000000,A=1.000000)" "(R=0.000000,G=1.000000,B=0.000000,A=1.000000)" 3.0))
            (if (Variables|Default|GetRampeIsInPositioning?)
              (Transformation|SetWorldTransform (Variables|Default|GetDefaultSceneRoot (.NewRampe (Variables|Default|GetNewRampe))) (Math|Transform|MakeTransform (.Location (Collision|BreakHitResult _outhit)) (Math|Rotator|MakeRotationfromAxes (Math|Vector|RotateVector (.Normal (Collision|BreakHitResult _outhit)) (Math|Vector|RotatorfromAxisandAngle (Math|Vector|CrossProduct (.Normal (Collision|BreakHitResult _outhit)) (Math|Vector|Normalize (Math|Vector|ProjectVectorontoPlane (Math|Vector|GetForwardVector _returnvalue) (.Normal (Collision|BreakHitResult _outhit))))) 9e+01)) (Math|Vector|ProjectVectorontoPlane (Math|Vector|GetRightVector _returnvalue) (.Normal (Collision|BreakHitResult _outhit))) (.Normal (Collision|BreakHitResult _outhit)))) false false)
              (else
                (bind _returnvalue_3 (Game|SpawnActorfromClass 0 (Math|Transform|MakeTransform (.Location (Collision|BreakHitResult _outhit)) (Math|Rotator|MakeRotationfromAxes (Math|Vector|RotateVector (.Normal (Collision|BreakHitResult _outhit)) (Math|Vector|RotatorfromAxisandAngle (Math|Vector|CrossProduct (.Normal (Collision|BreakHitResult _outhit)) (Math|Vector|Normalize (Math|Vector|ProjectVectorontoPlane (Math|Vector|GetForwardVector _returnvalue) (.Normal (Collision|BreakHitResult _outhit))))) 9e+01)) (Math|Vector|ProjectVectorontoPlane (Math|Vector|GetRightVector _returnvalue) (.Normal (Collision|BreakHitResult _outhit))) (.Normal (Collision|BreakHitResult _outhit)))) "Undefined" 0 0))
                (Variables|Default|SetNewRampe 0 _returnvalue_3))))
          (:then_1
            (Utilities|FlowControl|DoOnce false :!label _label
              (:Completed
                (Variables|Default|SetRampeIsInPositioning? true))))))))
  (:Released
    (Utilities|FlowControl|Sequence
      (:then_0
        (Variables|Default|SetRampeIsInPositioning? false)
        (Timeline|Timeline_0 Stop))
      (:then_1
        (goto _label Reset))
      (:then_2
        (Utilities|FlowControl|Delay 4.0)
        (Actor|DestroyActor (.NewRampe (Variables|Default|GetNewRampe)))))))

(fn ConstructionScript)